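; Personaje is a player character Blueprint that handles basic movement, camera look and jumping.
; Input axes alante and derecha add movement along the control rotation's forward and right vectors, so movement follows where the controller faces.
; The mirar and girar axes feed controller pitch and yaw, and the saltar action triggers Jump.
; The BeginPlay, overlap, Tick and construction script graphs hold no logic.
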(event EventBeginPlay)

(event EventActorBeginOverlap
  (params (OtherActor :type Actor%20Object%20Reference)))

(event EventTick
  (params (DeltaSeconds :type Float%20%28single-precision%29)))

(event Input|ActionEvents|InputActionsaltar
  (params (Key :type Key%20Structure :default "AnyKey"))
  ;[1 1 1] Movimientos
  (:Pressed
    (Character|Jump)))

(event Input|AxisEvents|InputAxisalante
  (params (AxisValue :type Float%20%28single-precision%29))
  ;[1 1 1] Movimientos
  (Pawn|Input|AddMovementInput (Math|Vector|GetForwardVector (Pawn|GetControlRotation :!class /Script/Engine.Pawn)) AxisValue false))

(event Input|AxisEvents|InputAxisderecha
  (params (AxisValue :type Float%20%28single-precision%29))
  ;[1 1 1] Movimientos
  (Pawn|Input|AddMovementInput (Math|Vector|GetRightVector (Pawn|GetControlRotation :!class /Script/Engine.Pawn)) AxisValue false))

(event Input|AxisEvents|InputAxisgirar
  (params (AxisValue :type Float%20%28single-precision%29))
  ;[1 1 1] Movimientos
  (Pawn|Input|AddControllerYawInput AxisValue))

(event Input|AxisEvents|InputAxismirar
  (params (AxisValue :type Float%20%28single-precision%29))
  ;[1 1 1] Movimientos
  (Pawn|Input|AddControllerPitchInput AxisValue))

(fn ConstructionScript)