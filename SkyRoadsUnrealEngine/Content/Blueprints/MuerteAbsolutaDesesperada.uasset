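; MuerteAbsolutaDesesperada is a lethal obstacle that destroys the player pawn when a hit occurs at high speed.
; On Hit, it casts player pawn 0 to PersonajePrincipal and to SpaceInvader, checking each type's VelocidadActual against a fixed threshold.
; Exceeding that threshold destroys the pawn outright.
; The colliding actor is never checked, so any hit tests the player's current speed.
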(event EventBeginPlay)

(event EventActorBeginOverlap
  (params (OtherActor :type Actor%20Object%20Reference)))

(event EventTick
  (params (DeltaSeconds :type Float%20%28single-precision%29)))

(event Collision|EventHit
  (params (MyComp :type Primitive%20Component%20Object%20Reference) (Other :type Actor%20Object%20Reference) (OtherComp :type Primitive%20Component%20Object%20Reference) (bSelfMoved :type Boolean) (HitLocation :type Vector :default "0, 0, 0") (HitNormal :type Vector :default "0, 0, 0") (NormalImpulse :type Vector :default "0, 0, 0") (Hit :type Hit%20Result%20Structure%20%28by%20ref%29))
  (bind _returnvalue (Game|Player|GetPlayerPawn 0))
  (Utilities|FlowControl|Sequence
    (:then_0
      (bind _aspersonaje_principal (Utilities|Casting|CastToPersonajePrincipal _returnvalue))
      (if (> (Variables|/Game/Personaje/PersonajePrincipal.PersonajePrincipal_C|GetVelocidadActual _aspersonaje_principal) 6e+02)
        (Actor|DestroyActor _returnvalue :!label _label)))
    (:then_1
      (bind _asspace_invader (Utilities|Casting|CastToSpaceInvader _returnvalue))
      (if (> (Variables|/Game/Personaje/SpaceInvader.SpaceInvader_C|GetVelocidadActual _asspace_invader) 6e+02)
        (goto _label)))))

(fn ConstructionScript)