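; Frenar is an actor Blueprint that slows the player's SpaceInvader pawn after something hits it.
; Hit sets the Encima flag and ActorEndOverlap clears it; while it is set, Tick repeatedly lowers the pawn's max walk speed.
; Neither event checks which actor triggered it, and the nodes that would raise the speed again are disconnected, so the slowdown is never undone here.
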(event EventBeginPlay)

(event Collision|EventActorEndOverlap
  (params (OtherActor :type Actor%20Object%20Reference))
  (Variables|Default|Setencima false))

(event Collision|EventHit
  (params (MyComp :type Primitive%20Component%20Object%20Reference) (Other :type Actor%20Object%20Reference) (OtherComp :type Primitive%20Component%20Object%20Reference) (bSelfMoved :type Boolean) (HitLocation :type Vector :default "0, 0, 0") (HitNormal :type Vector :default "0, 0, 0") (NormalImpulse :type Vector :default "0, 0, 0") (Hit :type Hit%20Result%20Structure%20%28by%20ref%29))
  (Variables|Default|Setencima true))

(event EventTick
  (params (DeltaSeconds :type Float%20%28single-precision%29))
  (if (Variables|Default|Getencima)
    (bind _asspace_invader (Utilities|Casting|CastToSpaceInvader (Game|Player|GetPlayerPawn 0)))
    (Variables|/Script/Engine.CharacterMovementComponent|SetMaxWalkSpeed (Variables|/Script/Engine.Character|GetCharacterMovement _asspace_invader) 1e+02)))

(fn ConstructionScript)