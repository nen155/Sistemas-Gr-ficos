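; Player character Blueprint for a game with speed control, a fuel ratio, a timer and crash death.
; Holding W or S steps the current speed up or down each Tick, updating MaxWalkSpeed and the fuel ratio, while axis input moves along world +X.
; Hits at high X or any vertical velocity, filtered by impact height, destroy the actor and open the restart menu.
; It also creates the HUD, copies its remaining time, and toggles a map-selection widget with M.
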(event Custom|Muerte
  (Variables|/Script/Engine.PlayerController|SetbShowMouseCursor (Game|GetPlayerController 0) true)
  (bind _returnvalue (UserInterface|CreateWidget "/Game/MenuReinicio.MenuReinicio_C"))
  (UserInterface|Viewport|AddtoPlayerScreen _returnvalue))

(event EventBeginPlay
  (Viewport|RemoveAllWidgets)
  (bind _returnvalue (UserInterface|CreateWidget "/Game/HUD.HUD_C"))
  (UserInterface|Viewport|AddtoPlayerScreen _returnvalue)
  (EventDispatchers|BindEventtoOnDestroyed (delegate Custom|Muerte)))

(event EventActorBeginOverlap
  (params (OtherActor :type Actor%20Object%20Reference)))

(event EventTick
  (params (DeltaSeconds :type Float%20%28single-precision%29)))

(event EventTick
  (params (DeltaSeconds :type Float%20%28single-precision%29))
  (Utilities|FlowControl|Sequence
    (:then_0
      (if (Variables|Default|GetandarPresionado)
        (if (< (Variables|Default|GetVelocidadActual) (Variables|Default|GetVelocidadMaxima))
          (bind _output_get (Variables|Default|SetVelocidadActual (+ (Variables|Default|GetVelocidadActual) (Variables|Default|GetaddVelocidad))))
          (Variables|/Script/Engine.CharacterMovementComponent|SetMaxWalkSpeed (Variables|Character|GetCharacterMovement) (* _output_get 1e+01))
          (Variables|Default|SetproporcionCombustible (/ _output_get 1e+01)))))
    (:then_1
      (if (Variables|Default|GetpararPresionado)
        (if (< 0.0 (Variables|Default|GetVelocidadActual))
          (bind _output_get_2 (Variables|Default|SetVelocidadActual (- (Variables|Default|GetVelocidadActual) (Variables|Default|GetrestarVelocidad))))
          (Variables|/Script/Engine.CharacterMovementComponent|SetMaxWalkSpeed (Variables|Character|GetCharacterMovement) (* _output_get_2 1e+01))
          (Variables|Default|SetproporcionCombustible (/ _output_get_2 1e+01)))))
    (:then_2
      (Variables|Default|SettiempoEmpleado (Variables|/Game/HUD.HUD_C|GetTimeLeft (stale EventBeginPlay _returnvalue))))))

(event Collision|EventHit
  (params (MyComp :type Primitive%20Component%20Object%20Reference) (Other :type Actor%20Object%20Reference) (OtherComp :type Primitive%20Component%20Object%20Reference) (bSelfMoved :type Boolean) (HitLocation :type Vector) (HitNormal :type Vector :default "0, 0, 0") (NormalImpulse :type Vector :default "0, 0, 0") (Hit :type Hit%20Result%20Structure%20%28by%20ref%29))
  (bind _returnvalue (Transformation|GetVelocity))
  (bind (_x _y _z) (Math|Vector|BreakVector _returnvalue))
  (if (!= (.Z (Math|Vector|BreakVector HitLocation)) 2e+01)
    (if (or (>= _x 5e+02) (!= _z 0.0))
      (Actor|DestroyActor))))

(event Input|AxisEvents|InputAxisAndar
  (params (AxisValue :type Float%20%28single-precision%29))
  (Pawn|Input|AddMovementInput (Math|Vector|GetForwardVector "0, 0, 0") AxisValue false))

(event Input|KeyboardEvents|M
  (params (Key :type Key%20Structure :default "AnyKey"))
  (bind _returnvalue (Game|GetPlayerController 0))
  (:Pressed
    (Utilities|FlowControl|FlipFlop
      (:A
        (Variables|/Script/Engine.PlayerController|SetbShowMouseCursor _returnvalue true)
        (bind _returnvalue_2 (UserInterface|CreateWidget "/Game/ElegirMapa.ElegirMapa_C"))
        (UserInterface|Viewport|AddtoPlayerScreen _returnvalue_2))
      (:B
        (Variables|/Script/Engine.PlayerController|SetbShowMouseCursor _returnvalue false)
        (Class|VictoryBPFunctionLibrary|RemoveAllWidgetsOfClass "/Game/ElegirMapa.ElegirMapa_C")))))

(event Input|KeyboardEvents|W
  (params (Key :type Key%20Structure :default "AnyKey"))
  (:Pressed
    (Variables|Default|SetandarPresionado true))
  (:Released
    (Variables|Default|SetandarPresionado false)))

(event Input|KeyboardEvents|S
  (params (Key :type Key%20Structure :default "AnyKey"))
  (:Pressed
    (Variables|Default|SetpararPresionado true))
  (:Released
    (Variables|Default|SetpararPresionado false)))

(fn ConstructionScript)