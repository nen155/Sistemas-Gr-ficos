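; BP_Railing is a modular railing whose length is set by the RailLength variable.
; The construction script adds one static mesh component per segment, spaced evenly along local Y, and skips everything when RailLength is zero or less.
; After adding the segments, it moves the RailEnd component to cap the far end of the run.
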(fn ConstructionScript
  (if (> (Variables|DemoProperties|GetRail%20length) 0) ; Don't spawn any meshes if none are needed
    (for _index (range 1 (Variables|DemoProperties|GetRail%20length)) ; Repeat once for every mesh to spawn
      (bind _returnvalue (AddComponent|AddStaticMeshComponent false))
      (Transformation|SetRelativeLocation _returnvalue (Math|Vector|MakeVector 0.0 (* (- _index 1) 1.5e+02) 0.0) false))
    (Transformation|SetRelativeLocation (Variables|Default|GetRail%20end) (Math|Vector|MakeVector 0.0 (* (Variables|DemoProperties|GetRail%20length) 1.5e+02) 0.0) false)))