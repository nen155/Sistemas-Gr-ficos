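; Metal sphere actor that reacts to heat and water sent through the ElementalDamage interface event, with steam and hiss when the two meet.
; Tick decays Heat (faster when wet) and Wetness while Heat accumulates into Burntness, feeding all three to a dynamic material created in the construction script.
; Heat also drives smoke and looping-audio volume, while Wetness toggles drip effects and audio through paired DoOnce nodes that reset each other.
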(event Custom|Play%20Drip%20Audio
  (bind _dripping_audio (Variables|Audio|GetDripping%20Audio))
  ;[1 1 1] Dripping Audio
  (Utilities|FlowControl|DoOnce false
    (:Completed
      (Audio|Components|Audio|Play _dripping_audio 0.0)
      (Components|Activation|SetActive (Variables|BP_Metal_Sphere|GetDrips) true false) ; Turn on a dripping effect if wetness is above a certain value
      (Utilities|FlowControl|DoOnce false) ; enters at Reset
    )))

(event Custom|Stop%20Drip%20Audio
  (bind _dripping_audio (Variables|Audio|GetDripping%20Audio))
  ;[1 1 1] Dripping Audio
  (Utilities|FlowControl|DoOnce false
    (:Completed
      (Audio|Components|Audio|FadeOut _dripping_audio 1.0 0.0 :!class /Script/Engine.AudioComponent)
      (Components|Activation|SetActive (Variables|BP_Metal_Sphere|GetDrips) false false) ; Turn on a dripping effect if wetness is above a certain value
      (Utilities|FlowControl|DoOnce false) ; enters at Reset
    )))

(event EventElementalDamage
  (params (Heat :type Float%20%28single-precision%29) (Water :type Float%20%28single-precision%29))
  (bind _returnvalue (Transformation|GetActorLocation))
  (if (or (and (> (Variables|Default|GetHeat) 0.05) (> Water 0.0)) (and (> Heat 0.0) (> (Variables|Default|GetWetness) 0.2)))
    (Effects|SpawnEmitteratLocation "/Game/Assets/Effects/P_Steam_Puff.P_Steam_Puff" _returnvalue) ; Spawn a steam puff effect
    (Audio|PlaySoundatLocation "/Game/Assets/Audio/WaterWeapon_ImpactSizzle_Cue.WaterWeapon_ImpactSizzle_Cue" _returnvalue 1.0 1.0) ; Steam hiss sound
  )
  (Variables|Default|SetHeat (Math|Float|Clamp(Float) (+ (Variables|Default|GetHeat) (* Heat 0.1))))
  (Variables|Default|SetWetness (Math|Float|Clamp(Float) (+ (Variables|Default|GetWetness) Water))))

(event EventTick
  (params (DeltaSeconds :type Float%20%28single-precision%29))
  (bind _metal_material (Variables|Default|GetMetal%20material))
  (Variables|Default|SetDelta%20seconds DeltaSeconds) ; Set the time between frames for use with interp nodes
  (Variables|Default|SetHeat (Math|Interpolation|FInterpTo (Variables|Default|GetHeat) 0.0 (Variables|Default|GetDelta%20seconds) (+ (Variables|Default|GetWetness) 0.25)))
  (Variables|Default|SetBurntness (Math|Float|Clamp(Float) (Math|Interpolation|FInterpTo (Variables|Default|GetBurntness) (+ (Variables|Default|GetBurntness) (Variables|Default|GetHeat)) (Variables|Default|GetDelta%20seconds) 0.15)))
  (Variables|Default|SetWetness (Math|Interpolation|FInterpTo (Variables|Default|GetWetness) 0.0 (Variables|Default|GetDelta%20seconds) 0.3))
  (Rendering|Material|SetScalarParameterValue _metal_material "Burntness" (Variables|Default|GetBurntness) :!class /Script/Engine.MaterialInstanceDynamic) ; Float values are used to drive various material effects
  (Rendering|Material|SetScalarParameterValue _metal_material "Heat" (Variables|Default|GetHeat) :!class /Script/Engine.MaterialInstanceDynamic)
  (Rendering|Material|SetScalarParameterValue _metal_material "Wetness" (Variables|Default|GetWetness) :!class /Script/Engine.MaterialInstanceDynamic)
  (Components|Activation|SetActive (Variables|Default|GetSmoke) (> (Variables|Default|GetHeat) 0.15) false) ; Turn on a smoke effect if heat is above a certain value
  (if (> (Variables|Default|GetWetness) 0.2)
    (CallFunction|PlayDripAudio)
    (else
      (CallFunction|StopDripAudio)))
  (Audio|Components|Audio|SetVolumeMultiplier (Variables|Audio|GetHeated%20Audio) (Math|Float|Lerp 0.0 0.5 (Variables|Default|GetHeat)) :!class /Script/Engine.AudioComponent))

(event EventBeginPlay
  (Audio|Components|Audio|Play (Variables|Audio|GetCooling%20Audio) 0.0))

(fn ConstructionScript
  (bind _returnvalue (Rendering|Material|CreateDynamicMaterialInstance (Variables|Default|GetMetal%20sphere) 0 0 :!class /Script/Engine.PrimitiveComponent))
  (Variables|Default|SetMetal%20material _returnvalue))