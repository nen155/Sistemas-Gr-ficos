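; Basic light bulb Blueprint that can be toggled on and off with flash and sound.
; Turning on plays audio and a flash timeline whose value drives brightness of a warm color; turning off stops both, plays a switch-off cue and sets black.
; UpdateLightColor applies the color to the light and two dynamic bulb materials created in the construction script, using alpha to scale intensity.
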(event EventToggle
  (params (On/off :type Boolean))
  (bind _light_audio (Variables|Audio|GetLight%20Audio))
  (if On/off
    (Audio|Components|Audio|Play _light_audio 0.0)
    (bind _flash (Timeline|Light%20flash PlayFromStart)
      (:Update
        (CallFunction|UpdateLightColor (Math|Color|MakeColor 1.0 0.7 0.3 _flash)) ; Custom function updates the color of the light component and light bulb materials
      ))
    (else
      (Utilities|FlowControl|Sequence ; Interrupt timeline before turning off
        (:then_0
          (Timeline|Light%20flash Stop))
        (:then_1
          (Audio|Components|Audio|Stop _light_audio)
          (Class|GameplayStatics|PlaySoundAttached "/Game/Assets/Audio/Communication_LightOff_Cue.Communication_LightOff_Cue" _light_audio "None" "0, 0, 0" "EAttachLocation::KeepRelativeOffset" false 1.0 1.0)
          (CallFunction|UpdateLightColor) ; Change light color to black, effectively turning it off
        )))))

(fn ConstructionScript
  (bind _light_bulb (Variables|BP_Light_Bulb|GetLight%20bulb))
  (bind _returnvalue (Rendering|Material|CreateDynamicMaterialInstance _light_bulb 0 0 :!class /Script/Engine.PrimitiveComponent)) ; Create and apply Dynamic Material Instances for the light bulb mesh
  (Variables|Default|SetLight%20bulb%20material%201 _returnvalue)
  (bind _returnvalue_2 (Rendering|Material|CreateDynamicMaterialInstance _light_bulb 1 0 :!class /Script/Engine.PrimitiveComponent))
  (Variables|Default|SetLight%20bulb%20material%202 _returnvalue_2))

(fn UpdateLightColor
  (params (New%20color :type Linear%20Color%20Structure))
  (bind _light (Variables|BP_Light_Bulb|GetLight))
  (Rendering|Material|SetVectorParameterValue (Variables|Default|GetLight%20bulb%20material%202) "Emissive color" New%20color :!class /Script/Engine.MaterialInstanceDynamic)
  (Rendering|Components|Light|SetLightColor _light New%20color)
  (Rendering|Components|Light|SetIntensity _light (* (.A (Math|Color|BreakColor New%20color)) 2e+03)))